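; Player controller for multiplayer hitscan shooting from the player's follow camera.
; Shoot input passes a gate that limits the fire rate and runs a client line trace with debug drawing.
; On a hit, the trace endpoints go through server and multicast events (by naming), which re-trace and apply point damage to Player-tagged actors.
; A separate FireWeapon function, uncalled here, adds a muzzle flash to the trace.
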(event `self.ReceiveBeginPlay`
  (bind _asbp_player (cast `/Game/_Main/Blueprints/Player/BP_Player` (`self.K2_GetPawn`)))
  (set `self.Player Ref` _asbp_player))

(event `EnhancedInput|/Game/Input/Actions/IA_Shoot`
  (params (ActionValue :type Boolean) (ElapsedSeconds :type "Float (double-precision)") (TriggeredSeconds :type "Float (double-precision)") (InputAction :type "InputAction Object Reference" :default "/Game/Input/Actions/IA_Shoot.IA_Shoot"))
  (:`Triggered`
    (`/Engine/EditorBlueprintResources/StandardMacros.Gate` false :!label _label
      (:`Exit`
        (`|ExecutionSequence`
          (:`then_0`
            (goto _label :!via `Close`))
          (:`then_1`
            (`self.ClientLineTrace`)
            (`KismetSystemLibrary.Delay` 0.2)
            (goto _label :!via `Open`)))))))

(event `ClientLineTrace`
  (bind _player_ref (`self.Player Ref`))
  (bind _followcamera (`FocusMultiplayerGameCharacter.FollowCamera` _player_ref))
  (bind _returnvalue (`SceneComponent.K2_GetComponentLocation` _followcamera))
  (bind _returnvalue_2 (+ _returnvalue (* (`SceneComponent.GetForwardVector` _followcamera) (`self.BulletRange`))))
  (bind (_outhit _returnvalue_3) (`KismetSystemLibrary.LineTraceSingle` _returnvalue _returnvalue_2 "TraceTypeQuery1" false (`|MakeArray` _player_ref :!type "Actor Object Reference") "ForDuration"))
  (if _returnvalue_3
    (`self.ROS_LineTrace` _returnvalue _returnvalue_2 _player_ref)))

(event `ROS_LineTrace`
  (params (StartTrace :type "Vector Structure") (EndTrace :type "Vector Structure") (Instigator :type "Actor Object Reference"))
  (`self.MC_LineTrace` StartTrace EndTrace Instigator))

(event `MC_LineTrace`
  (params (`Start Trace` :type "Vector Structure") (`End Trace` :type "Vector Structure") (Instigator :type "Actor Object Reference"))
  (bind (_outhit _returnvalue) (`KismetSystemLibrary.LineTraceSingle` `Start Trace` `End Trace` "TraceTypeQuery1" false (`|MakeArray` Instigator)))
  (bind (_bblockinghit _binitialoverlap _time _distance _location _impactpoint _normal _impactnormal _physmat _hitactor) (`GameplayStatics.BreakHitResult` _outhit))
  (`/Engine/EditorBlueprintResources/StandardMacros.IsValid` _hitactor
    (:`Is Valid`
      (if (and _returnvalue (`self.ActorHasTag` _hitactor "Player"))
        (`GameplayStatics.ApplyPointDamage` _hitactor (`self.Base Damage`) _impactnormal _outhit self (`self.Player Ref`) "/Script/Engine.DamageType")))))

(fn `FireWeapon`
  (`self.ClientLineTrace`)
  (`GameplayStatics.SpawnEmitterAtLocation` "/Game/MilitaryWeapSilver/FX/P_AssaultRifle_MuzzleFlash.P_AssaultRifle_MuzzleFlash" (`SceneComponent.GetSocketLocation` (`/Game/_Main/Blueprints/Player/BP_Player.SKM_Weapon` (`self.Player Ref`)) "MuzzleFlash") (struct :`Yaw` 90.0)))

(fn `UserConstructionScript`)